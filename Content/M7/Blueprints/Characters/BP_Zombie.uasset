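; BP_Zombie is a zombie character that reacts to damage and death through bound events from its BPCHealth component.
; It attaches a looping-style idle sound to its mesh on BeginPlay and keeps a reference to it.
; Damage plays a hit montage, pausing the idle sound until blend out.
; Death calls Play Montage with no montage set, then immediately destroys the actor and sound component.
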(event Custom|ZombieDamage
  (Animation|Montage|PlayMontage (Variables|Character|GetMesh) "/Game/M7/Art/Characters/Zombie/Anim/AM_ZombieAttacked.AM_ZombieAttacked"
    (:then
      (Class|AudioComponent|SetPaused (Variables|Default|GetIdleSoundRef) true))
    (:OnBlendOut
      (Class|AudioComponent|SetPaused (Variables|Default|GetIdleSoundRef) false))))

(event Custom|ZombieDead
  (Animation|Montage|PlayMontage (Variables|Character|GetMesh) 0
    (:then
      (Actor|DestroyActor)
      (Components|DestroyComponent (Variables|Default|GetIdleSoundRef)))))

(event EventBeginPlay
  (bind _bpc_health (Variables|Default|GetBPC_Health))
  (EventDispatchers|BindEventtoOnHealthReduced _bpc_health (delegate Custom|ZombieDamage))
  (EventDispatchers|BindEventtoOnDeath _bpc_health (delegate Custom|ZombieDead))
  (bind _returnvalue (Audio|SpawnSoundAttached "/Game/M7/SFX/Zombie/S_ZombieIdle.S_ZombieIdle" (Variables|Character|GetMesh) "Neck" "0, 0, 0" "0, 0, 0" "KeepRelativeOffset" false 1.0 1.0 0.0 "/Game/M7/SFX/Zombie/SATT_Zombie.SATT_Zombie" 0))
  (Variables|Default|SetIdleSoundRef _returnvalue))

(fn ConstructionScript)