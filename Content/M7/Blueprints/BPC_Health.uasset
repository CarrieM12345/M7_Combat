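; BPC_Health is a health component that tracks current Health against MaxHealth, starting full on BeginPlay.
; IncreaseHealth and ReduceHealth ignore non-positive amounts and clamp the result between zero and MaxHealth.
; It broadcasts OnHealthIncreased on gains, and either OnHealthReduced or, at zero, OnDeath on losses.
; No dead state is stored, so further damage at zero broadcasts OnDeath again.
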(event EventBeginPlay
  (Variables|Default|SetHealth (Variables|Default|GetMaxHealth)))

(fn IncreaseHealth
  (params (HealthAmount :type Float%20%28double-precision%29))
  (if (> HealthAmount 0.0)
    (Variables|Default|SetHealth (Math|Float|Clamp(Float) (+ HealthAmount (Variables|Default|GetHealth)) 0.0 (Variables|Default|GetMaxHealth)))
    (Default|CallOnHealthIncreased)))

(fn ReduceHealth
  (params (HealthAmount :type Float%20%28double-precision%29))
  (if (> HealthAmount 0.0)
    (bind _output_get (Variables|Default|SetHealth (Math|Float|Clamp(Float) (- (Variables|Default|GetHealth) HealthAmount) 0.0 (Variables|Default|GetMaxHealth))))
    (if (<= _output_get 0.0)
      (Default|CallOnDeath)
      (else
        (Default|CallOnHealthReduced)))))